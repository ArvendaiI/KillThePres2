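; Touch-controlled sniper pawn that aims within a clamped view cone, zooms by dividing FOV by Distance, and slows drag-look as zoom increases.
; Shooting line-traces from the camera, ragdolls and kills static or walking targets, and detects headshots by bone name; a timed mesh nudge fakes recoil.
; Outside training, headshots are saved to the GameInstance and a kill ends the level, swapping to Main_Character with an end screen.
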(event Custom|Input_Event
  (bind _distance (Variables|Default|GetDistance))
  (bind _returnvalue (* _distance 1e+01))
  (bind _returnvalue_2 (+ _returnvalue 1e+01))
  ;[1 1 1] Инпут
  (Pawn|Input|AddControllerYawInput (/ (.x (- (Math|Vector2D|MakeVector2D (.x (stale Input|TouchEvents|InputTouch Location)) (.y (stale Input|TouchEvents|InputTouch Location))) (Variables|Default|GetVector))) _returnvalue_2))
  (Pawn|Input|AddControllerPitchInput (/ (.y (- (Math|Vector2D|MakeVector2D (.x (stale Input|TouchEvents|InputTouch Location)) (.y (stale Input|TouchEvents|InputTouch Location))) (Variables|Default|GetVector))) _returnvalue_2)))

(event Custom|Loop
  ;[1 1 1] Приближение
  (Camera|SetFieldOfView (Variables|Default|GetCamera) (/ 9e+01 (Variables|Default|GetDistance))))

(event Custom|Shoot
  (bind _returnvalue (Game|GetPlayerCameraManager 0))
  (bind _returnvalue_2 (Transformation|GetActorLocation _returnvalue))
  ;[1 1 1] Shoot
  (bind (_outhit _returnvalue_3) (Collision|LineTraceByChannel _returnvalue_2 (+ _returnvalue_2 (* (Math|Vector|GetForwardVector (Variables|/Script/Engine.PlayerCameraManager|GetTransformComponent _returnvalue)) 2e+04)) "TraceTypeQuery1" false 0 "ForDuration"))
  (if _returnvalue_3
    (Utilities|FlowControl|Sequence
      (:then_0
        (bind _astarget_blueprint (Utilities|Casting|CastToTarget_Blueprint (.HitActor (Collision|BreakHitResult _outhit))))
        (Physics|SetSimulatePhysics (Variables|/Game/Game/Blueprints/Main/Target_Blueprint.Target_Blueprint_C|GetSkeletalMesh _astarget_blueprint) true)
        (Default|Killed _astarget_blueprint))
      (:then_1
        (bind _astarget_walk_bp (Utilities|Casting|CastToTarget_WalkBP (.HitActor (Collision|BreakHitResult _outhit))))
        (Physics|SetSimulatePhysics (Variables|/Game/Game/Blueprints/Main/Target_WalkBP.Target_WalkBP_C|GetSkeletalMesh _astarget_walk_bp) true)
        (Default|Killed _astarget_walk_bp)))
    (Utilities|FlowControl|Sequence
      (:then_0
        (if (Utilities|Name|Equal(Name) (.HitBoneName (Collision|BreakHitResult _outhit)) "BipTrump-Head")
          (CallFunction|HeadShotFunction)
          (if (not (Variables|/Game/Game/Blueprints/Main/MainGameInstance.MainGameInstance_C|GetTrening_Level (Variables|Default|GetGI)))
            (Variables|/Game/Game/Blueprints/Main/MainGameInstance.MainGameInstance_C|SetHeadShoot (Variables|Default|GetGI) true))))
      (:then_1
        (if (not (Variables|/Game/Game/Blueprints/Main/MainGameInstance.MainGameInstance_C|GetTrening_Level (Variables|Default|GetGI)))
          ;;[1 1 1] Задержка, помни что нужно переписать
          (Utilities|FlowControl|Delay 0.2)
          (CallFunction|EndLevel))))))

(event Custom|Shoot_Anim
  (bind _staticmesh (Variables|Default|GetStaticMesh))
  (bind _returnvalue (Transformation|GetWorldTransform _staticmesh))
  (bind _returnvalue_2 (Transformation|GetWorldTransform _staticmesh))
  (bind (_location _rotation) (Math|Transform|BreakTransform _returnvalue))
  (bind (_location_2 _rotation_2) (Math|Transform|BreakTransform _returnvalue_2))
  (bind (_x _y _z) (Math|Vector|BreakVector _location))
  (bind (_roll _pitch _yaw) (Math|Rotator|BreakRotator _rotation))
  (bind (_x_2 _y_2 _z_2) (Math|Vector|BreakVector _location_2))
  (bind (_roll_2 _pitch_2 _yaw_2) (Math|Rotator|BreakRotator _rotation_2))
  ;[1 1 1] Animation
  (Transformation|SetWorldTransform _staticmesh (Math|Transform|MakeTransform (Math|Vector|MakeVector (- _x_2 25.0) _y_2 _z_2) (Math|Rotator|MakeRotator _roll_2 (+ _pitch_2 12.0) _yaw_2)) false false)
  (Utilities|FlowControl|Delay 0.15)
  (Transformation|SetWorldTransform _staticmesh (Math|Transform|MakeTransform (Math|Vector|MakeVector (+ _x 25.0) _y _z) (Math|Rotator|MakeRotator _roll (- _pitch 12.0) _yaw)) false false))

(event Custom|End_Level
  (bind _returnvalue (Game|SpawnActorfromClass "/Game/Game/Blueprints/Main/Main_Character.Main_Character_C" (Transformation|GetWorldTransform (Variables|Default|GetDefaultSceneRoot)) "Undefined" 0 0))
  (Pawn|Possess (Game|GetPlayerController 0) _returnvalue)
  (bind _returnvalue_2 (UserInterface|CreateWidget "/Game/Game/Widget/InGame/EndLevel.EndLevel_C"))
  (UserInterface|Viewport|AddtoViewport _returnvalue_2 0)
  (Widget|RemovefromParent (Variables|Default|GetWidget_Control))
  ;[1 1 1] Нужно плавное возвращение к стандарту, возможно с наводом камеры на игрока или на жертву
  (Variables|Default|SetDistance 1.0)
  (Actor|DestroyActor))

(event EventBeginPlay
  (bind _returnvalue (Game|GetPlayerCameraManager 0))
  (bind _asmain_game_instance (Utilities|Casting|CastToMainGameInstance (Game|GetGameInstance)))
  (Variables|Default|SetGI _asmain_game_instance)
  (Variables|Default|SetStandartPos (.yaw (Transformation|GetWorldRotation (Variables|Default|GetCamera))))
  (bind _returnvalue_2 (UserInterface|CreateWidget "/Game/Game/Widget/InGame/Control_Widget.Control_Widget_C"))
  (Variables|Default|SetWidget_Control _returnvalue_2)
  (UserInterface|Viewport|AddtoViewport (Variables|Default|GetWidget_Control) 0)
  (bind _returnvalue_3 (UserInterface|CreateWidget "/Game/Game/Widget/InGame/HeadShotWidget.HeadShotWidget_C"))
  (Variables|Default|SetHeadShot_Var _returnvalue_3)
  (Variables|/Script/Engine.PlayerCameraManager|SetViewPitchMin _returnvalue -45.0)
  (Variables|/Script/Engine.PlayerCameraManager|SetViewPitchMax _returnvalue 45.0)
  (Variables|/Script/Engine.PlayerCameraManager|SetViewYawMin _returnvalue (- (Variables|Default|GetStandartPos) 6e+01))
  (Variables|/Script/Engine.PlayerCameraManager|SetViewYawMax _returnvalue (+ (Variables|Default|GetStandartPos) 6e+01)))

(event Input|KeyboardEvents|R
  (params (Key :type Key%20Structure :default "None"))
  (:Pressed
    (Utilities|FlowControl|FlipFlop
      (:A
        (Components|StaticMesh|SetStaticMesh (Variables|Default|GetStaticMesh) "/Game/AssetsvilleTown/Meshes/Weapons/SM_Rifle_02.SM_Rifle_02"))
      (:B
        (Components|StaticMesh|SetStaticMesh (Variables|Default|GetStaticMesh) "/Game/AssetsvilleTown/Meshes/Weapons/SM_Rifle_03.SM_Rifle_03")))))

(event Input|TouchEvents|InputTouch
  (params (Location :type Vector) (FingerIndex :type ETouchIndex%20Enum))
  ;[1 1 1] Инпут
  (:Pressed
    (Variables|Default|SetVector (Math|Vector2D|MakeVector2D (.x Location) (.y Location)) :!label _label))
  (:Released
    (goto _label))
  (:Moved
    (if (> (.x Location) 3e+02)
      (CallFunction|InputEvent)
      (goto _label))))

(fn ConstructionScript)

(fn HeadShotFunction
  (if (UserInterface|Viewport|IsinViewport (Variables|Default|GetHeadShot_Var))
    (Variables|/Game/Game/Widget/InGame/HeadShotWidget.HeadShotWidget_C|SetTimer (Variables|Default|GetHeadShot_Var) 2.0)
    (else
      (UserInterface|Viewport|AddtoViewport (Variables|Default|GetHeadShot_Var) 0))))