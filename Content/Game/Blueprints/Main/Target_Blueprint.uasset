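; Target Blueprint whose Killed event records level completion in the game instance when the target is killed.
; BeginPlay caches the MainGameInstance, and Killed runs a sequence of checks on its level flags.
; Levels 1 and 2 set their finish flags to true, while level 3 sets FinishLevel4 to false.
; The Level4 check has no action attached, and nothing in this Blueprint calls Killed.
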(event Custom|Killed
  ;[1 1 1] Эвент завершения игры
  (Utilities|FlowControl|Sequence
    (:then_0
      (if (Variables|/Game/Game/Blueprints/Main/MainGameInstance.MainGameInstance_C|GetOn_Level%201 (Variables|Default|GetGI))
        (Variables|/Game/Game/Blueprints/Main/MainGameInstance.MainGameInstance_C|SetFinish_Level_1 (Variables|Default|GetGI) true)))
    (:then_1
      (if (Variables|/Game/Game/Blueprints/Main/MainGameInstance.MainGameInstance_C|GetOn_Level%202 (Variables|Default|GetGI))
        (Variables|/Game/Game/Blueprints/Main/MainGameInstance.MainGameInstance_C|SetFinish_Level_2 (Variables|Default|GetGI) true)))
    (:then_2
      (if (Variables|/Game/Game/Blueprints/Main/MainGameInstance.MainGameInstance_C|GetOn_Level%203 (Variables|Default|GetGI))
        (Variables|/Game/Game/Blueprints/Main/MainGameInstance.MainGameInstance_C|SetFinish_Level_4 (Variables|Default|GetGI) false)))
    (:then_3
      (if (Variables|/Game/Game/Blueprints/Main/MainGameInstance.MainGameInstance_C|GetLevel_4 (Variables|Default|GetGI))
        _))))

(event EventBeginPlay
  (bind _asmain_game_instance (Utilities|Casting|CastToMainGameInstance (Game|GetGameInstance)))
  (Variables|Default|SetGI _asmain_game_instance))

(fn ConstructionScript)