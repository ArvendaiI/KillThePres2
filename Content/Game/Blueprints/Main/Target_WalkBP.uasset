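; Walking target actor whose death marks the current level (one of six) as finished in MainGameInstance.
; It registers itself with the game instance on BeginPlay, and Start_Walk and Stop_Walk toggle a Walk multiplier that selects looping walk or idle animation.
; Tick slides the skeletal mesh along its right vector without sweep, while separate events turn it by fixed yaw steps.
; Killed blocks further movement and rotation.
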(event Custom|Killed
  ;[1 1 1] Эвент завершения игры
  (Variables|Default|SetKilled_Var true)
  (Utilities|FlowControl|Sequence
    (:then_0
      (if (Variables|/Game/Game/Blueprints/Main/MainGameInstance.MainGameInstance_C|GetOn_Level%201 (Variables|Default|GetGI))
        (Variables|/Game/Game/Blueprints/Main/MainGameInstance.MainGameInstance_C|SetFinish_Level_1 (Variables|Default|GetGI) true)))
    (:then_1
      (if (Variables|/Game/Game/Blueprints/Main/MainGameInstance.MainGameInstance_C|GetOn_Level%202 (Variables|Default|GetGI))
        (Variables|/Game/Game/Blueprints/Main/MainGameInstance.MainGameInstance_C|SetFinish_Level_2 (Variables|Default|GetGI) true)))
    (:then_2
      (if (Variables|/Game/Game/Blueprints/Main/MainGameInstance.MainGameInstance_C|GetOn_Level%203 (Variables|Default|GetGI))
        (Variables|/Game/Game/Blueprints/Main/MainGameInstance.MainGameInstance_C|SetFinish_Level_3 (Variables|Default|GetGI) true)))
    (:then_3
      (if (Variables|/Game/Game/Blueprints/Main/MainGameInstance.MainGameInstance_C|GetLevel_4 (Variables|Default|GetGI))
        (Variables|/Game/Game/Blueprints/Main/MainGameInstance.MainGameInstance_C|SetFinish_Level_4 (Variables|Default|GetGI) true)))
    (:then_4
      (if (Variables|/Game/Game/Blueprints/Main/MainGameInstance.MainGameInstance_C|GetLevel_5 (Variables|Default|GetGI))
        (Variables|/Game/Game/Blueprints/Main/MainGameInstance.MainGameInstance_C|SetFinish_Level_5 (Variables|Default|GetGI) true)))
    (:then_5
      (if (Variables|/Game/Game/Blueprints/Main/MainGameInstance.MainGameInstance_C|GetLevel_6 (Variables|Default|GetGI))
        (Variables|/Game/Game/Blueprints/Main/MainGameInstance.MainGameInstance_C|SetFinish_Level_6 (Variables|Default|GetGI) true)))))

(event Custom|Animation
  (if (> (Variables|Default|GetWalk) 0.0)
    (Components|Animation|PlayAnimation (Variables|Default|GetSkeletalMesh) "/Game/Game/Assets/MainTarget/Walk_Anim.Walk_Anim" true)
    (else
      (Components|Animation|PlayAnimation (Variables|Default|GetSkeletalMesh) "/Game/Game/Assets/MainTarget/Idle_Anim.Idle_Anim" true))))

(event Custom|Stop_Walk
  (Variables|Default|SetWalk 0.0)
  (CallFunction|Animation))

(event Custom|Rotate_Event
  (if (not (Variables|Default|GetKilled_Var))
    (Transformation|AddRelativeRotation (Variables|Default|GetSkeletalMesh) "0,-45.000000, 0" false false)))

(event Custom|Start_Walk
  (Variables|Default|SetWalk 1.0)
  (CallFunction|Animation))

(event Custom|Rotate_Event_2
  (if (not (Variables|Default|GetKilled_Var))
    (Transformation|AddRelativeRotation (Variables|Default|GetSkeletalMesh) "0,90.000000, 0" false false)))

(event Custom|Rotate_Event3
  (if (not (Variables|Default|GetKilled_Var))
    (Transformation|AddRelativeRotation (Variables|Default|GetSkeletalMesh) "0.000000,-15.000000, 0" false false)))

(event EventTick
  (params (DeltaSeconds :type Float%20%28single-precision%29))
  (if (not (Variables|Default|GetKilled_Var))
    (Transformation|AddRelativeLocation (Variables|Default|GetSkeletalMesh) (* (Math|Vector|GetRightVector (Variables|Default|GetSkeletalMesh)) (* DeltaSeconds 1.2e+02 (Variables|Default|GetWalk))) false false)))

(event EventBeginPlay
  (bind _asmain_game_instance (Utilities|Casting|CastToMainGameInstance (Game|GetGameInstance)))
  (Variables|Default|SetGI _asmain_game_instance)
  (CallFunction|Animation)
  (Variables|Default|SetTarget self)
  (Variables|Default|SetKilled_Var false)
  (Variables|/Game/Game/Blueprints/Main/MainGameInstance.MainGameInstance_C|SetTarget_Walk_War (Variables|Default|GetGI) (Variables|Default|GetTarget)))

(fn ConstructionScript)