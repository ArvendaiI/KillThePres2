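; Game instance Blueprint that opens the main menu and level selection screens and holds level selection flags.
; CreateMM and SelectLevel each create their widget, store a reference to it and add it to the viewport.
; Diselect clears the flags for the six levels and the training level.
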(event Custom|CreateMM
  (bind _returnvalue (UserInterface|CreateWidget "/Game/Game/Widget/Main_Menu/Main_MenuW.Main_MenuW_C"))
  (Variables|Default|SetMainMenu _returnvalue)
  (UserInterface|Viewport|AddtoViewport (Variables|Default|GetMainMenu) 0))

(event Custom|SelectLevel
  (bind _returnvalue (UserInterface|CreateWidget "/Game/Game/Widget/Main_Menu/SelectLevel.SelectLevel_C"))
  (Variables|Default|SetSelectLevelV _returnvalue)
  (UserInterface|Viewport|AddtoViewport (Variables|Default|GetSelectLevelV) 0))

(event Custom|Diselect
  (Variables|Levels|SetLevel_1 false)
  (Variables|Levels|SetLevel_2 false)
  (Variables|Levels|SetLevel_3 false)
  (Variables|Levels|SetLevel_4 false)
  (Variables|Levels|SetLevel_5 false)
  (Variables|Levels|SetLevel_6 false)
  (Variables|Levels|SetTrening_Level false))